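; Arkanoid menu ball that flies along its forward vector, with sound feedback for hits and death.
; Tick offsets the actor by Speed scaled by delta time, without sweep, then calls Move with zero.
; BeginPlay binds a delegate to OnDeadEvent.
; Hit plays a sine ping, and DeadEffect plays a teleport sound, both as 2D audio.
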(event EventBeginPlay
  (EventDispatchers|BindEventtoOnDeadEvent (EventDispatchers|CreateEvent :!event DeadEffect)))

(event EventTick
  (params (DeltaSeconds :type Float%20%28single-precision%29))
  (Transformation|AddActorWorldOffset (* (* DeltaSeconds (Variables|Default|GetSpeed)) (Transformation|GetActorForwardVector)))
  (Class|Ball|Move 0.0))

(event Collision|EventHit
  (params (MyComp :type Primitive%20Component%20Object%20Reference) (Other :type Actor%20Object%20Reference) (OtherComp :type Primitive%20Component%20Object%20Reference) (bSelfMoved :type Boolean) (HitLocation :type Vector :default "0, 0, 0") (HitNormal :type Vector :default "0, 0, 0") (NormalImpulse :type Vector :default "0, 0, 0") (Hit :type Hit%20Result%20Structure%20%28by%20ref%29))
  (Audio|PlaySound2D "/Engine/EngineSounds/1kSineTonePing.1kSineTonePing" 1.0 1.0 0.0 0 0))

(fn ConstructionScript)

(fn DeadEffect
  (Audio|PlaySound2D "/Engine/VREditor/Sounds/UI/Teleport_Committed.Teleport_Committed" 1.0 1.0 0.0 0 0))